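; P-38 plane pawn that flies forward continuously while the player steers pitch and roll.
; Tick adds forward movement input and spins the Left and Right propellers through RotatePropeller, scaled by delta time and PropellerSpeed.
; The propeller calls are chained and re-entered from several Sequence pins, including one behind a Delay, so they can run more than once per frame.
; Clamped Pitch and Roll axes apply local rotation scaled by delta time and PlayerRotateSpeed.
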(event EventTick
  (params (DeltaSeconds :type Float%20%28single-precision%29))
  ;[1 1 1] 이동
  (Utilities|FlowControl|Sequence
    (:then_0
      ;;[1 1 1] 앞으로 이동
      (Pawn|Input|AddMovementInput (Transformation|GetActorForwardVector) 1.0 false)
      (Utilities|FlowControl|Delay 3.0)
      ;;[1 1 1] 프로펠러 회전
      (CallFunction|RotatePropeller (Variables|Default|GetLeft) :!label _label))
    (:then_1
      (goto _label))
    (:then_2
      _))
  (CallFunction|RotatePropeller (Variables|Default|GetRight)))

(event Input|AxisEvents|InputAxisPitch
  (params (AxisValue :type Float%20%28single-precision%29))
  ;[1 1 1] Pitch
  (Transformation|AddActorLocalRotation (Math|Rotator|MakeRotator 0.0 (* (Math|Float|Clamp(Float) AxisValue -1.0) (Utilities|Time|GetWorldDeltaSeconds) (Variables|Speed|GetPlayerRotateSpeed)) 0.0) false false))

(event Input|AxisEvents|InputAxisRoll
  (params (AxisValue :type Float%20%28single-precision%29))
  ;[1 1 1] Roll
  (Transformation|AddActorLocalRotation (Math|Rotator|MakeRotator (* (Math|Float|Clamp(Float) AxisValue -1.0) (Utilities|Time|GetWorldDeltaSeconds) (Variables|Speed|GetPlayerRotateSpeed)) 0.0 0.0) false false))

(fn ConstructionScript)

(fn RotatePropeller
  (params (Where :type Scene%20Component%20Object%20Reference))
  (Transformation|AddRelativeRotation Where (Math|Rotator|MakeRotator (* (Utilities|Time|GetWorldDeltaSeconds) (Variables|Default|GetPropellerSpeed)) 0.0 0.0) false false))