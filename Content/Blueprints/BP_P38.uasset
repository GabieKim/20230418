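; BP_P38 is a P-38 plane Blueprint that flies forward along world X and spins its left and right propellers.
; Each Tick, a Sequence applies the frame-time-scaled MoveSpeed offset and calls RotatePropeller, which adds roll scaled by PropellerSpeed.
; A three-second Delay after the movement also feeds the propeller calls, which overlap with the other Sequence branches.
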(event EventTick
  (params (DeltaSeconds :type Float%20%28single-precision%29))
  (Utilities|FlowControl|Sequence
    (:then_0
      ;[1 1 1] 앞으로 이동
      (Transformation|AddActorWorldOffset (Math|Vector|MakeVector (* (Utilities|Time|GetWorldDeltaSeconds) (Variables|Speed|GetMoveSpeed)) 0.0 0.0))
      (Utilities|FlowControl|Delay 3.0)
      ;[1 1 1] 프로펠러 회전
      (CallFunction|RotatePropeller (Variables|Default|GetLeft) :!label _label))
    (:then_1
      (goto _label))
    (:then_2
      _))
  (CallFunction|RotatePropeller (Variables|Default|GetRight)))

(fn ConstructionScript)

(fn RotatePropeller
  (params (Where :type Scene%20Component%20Object%20Reference))
  (Transformation|AddRelativeRotation Where (Math|Rotator|MakeRotator (* (Utilities|Time|GetWorldDeltaSeconds) (Variables|Default|GetPropellerSpeed)) 0.0 0.0) false false))